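; Tower_BP is an automated turret that tracks and shoots whatever actor enters its trigger volume.
; Overlap events set or clear the target lock, and Tick chooses between aiming and firing or an idle spin.
; RInterpTo smooths gun rotation, with pitch clamped while tracking.
; Firing spawns Projectile_BP at the barrel socket after a short Delay, which throttles the per-tick calls into a fire rate.
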(event `self.Trigger_Volume.OnComponentBeginOverlap`
  (params (OverlappedComponent :type "PrimitiveComponent Object Reference") (OtherActor :type "Actor Object Reference") (OtherComp :type "PrimitiveComponent Object Reference") (OtherBodyIndex :type Integer) (bFromSweep :type Boolean) (SweepResult :type "HitResult Structure (by ref)"))
  ;[1 1 1] When entering the towers attack radius, set the target to attack and the Target_Locked variable to true
  (set `self.Target` OtherActor)
  (set `self.Target_Locked` true))

(event `self.Trigger_Volume.OnComponentEndOverlap`
  (params (OverlappedComponent :type "PrimitiveComponent Object Reference") (OtherActor :type "Actor Object Reference") (OtherComp :type "PrimitiveComponent Object Reference") (OtherBodyIndex :type Integer))
  ;[1 1 1] When Exiting the towers attack area, set the Target_Locked variable to false.
  (set `self.Target_Locked` false))

(event `self.ReceiveTick`
  (params (DeltaSeconds :type "Float (single-precision)"))
  ;[1 1 1] Execute every tick
  (set `self.DeltaTime` DeltaSeconds)
  (if (`self.Target_Locked`)
    (`self.Update TurretRotation`)
    (`self.Fire_Turret`)
    (else
      (`self.Idle`))))

(event `Update TurretRotation`
  ;[1 1 1] Point the turret towards its target
  (`SceneComponent.K2_SetWorldRotation` (`self.Tower1_Gun`) (`KismetMathLibrary.RInterpTo` (`SceneComponent.K2_GetComponentRotation` (`self.Tower1_Gun`)) (`KismetMathLibrary.MakeRotator` 0.0 (`KismetMathLibrary.ClampAngle` (.pitch (`KismetMathLibrary.FindLookAtRotation` (`SceneComponent.K2_GetComponentLocation` (`self.Tower1_Gun`)) (`self.K2_GetActorLocation` (`self.Target`)))) -35.0 30.0) (.yaw (`KismetMathLibrary.FindLookAtRotation` (`SceneComponent.K2_GetComponentLocation` (`self.Tower1_Gun`)) (`self.K2_GetActorLocation` (`self.Target`))))) (`self.DeltaTime`) 5.0) false false))

(event `Idle`
  (bind _returnvalue (`SceneComponent.K2_GetComponentRotation` (`self.Tower1_Gun`)))
  ;[1 1 1] Idle state of the turret
  (`SceneComponent.K2_SetWorldRotation` (`self.Tower1_Gun`) (`KismetMathLibrary.RInterpTo` _returnvalue (`KismetMathLibrary.MakeRotator` 0.0 0.0 (+ (.yaw _returnvalue) 10.0)) (`self.DeltaTime`) 5.0) false false))

(event `Fire_Turret`
  (`KismetSystemLibrary.Delay` 0.2)
  (`|SpawnActorFromClass` "/Game/Tower+Projectile/Projectile_BP.Projectile_BP_C" (`SceneComponent.GetSocketTransform` (`self.Tower1_Gun`) "BarrelEND" "RTS_World") "Undefined" "OverrideRootScale" null null))

(fn `UserConstructionScript`)