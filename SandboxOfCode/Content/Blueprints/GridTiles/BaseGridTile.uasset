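; BaseGridTile is an actor that generates a flat grid of PlainGridTile actors when play begins.
; It takes the world location of its Tile component as the grid origin and passes its GridWidth and GridLength to FillGrid.
; FillGrid uses nested loops to spawn tiles at a fixed, hard-coded spacing along X and Y, then prints a completion message.
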(event `self.ReceiveBeginPlay`
  ;[1 1 1] Set the start position and then make a grid
  (set `self.SpawnStartLocation` (`SceneComponent.K2_GetComponentLocation` (`self.Tile`))) ; Get Start point
  (`self.FillGrid` (`self.GridWidth`) (`self.GridLength`)))

(event `FillGrid`
  (params (`Max Width` :type Integer :default 0) (`Max Length` :type Integer :default 0))
  ;[1 1 1] Generates a square grid of tiles
  (for _index (range (+ `Max Width` 1))
    (for _index_2 (range (+ `Max Length` 1))
      (`|SpawnActorFromClass` "/Game/Blueprints/GridTiles/PlainGridTile.PlainGridTile_C" (`KismetMathLibrary.Conv_VectorToTransform` (+ (`KismetMathLibrary.MakeVector` (* _index_2 200.0) (* _index 200.0)) (`self.SpawnStartLocation`))) "Undefined" "OverrideRootScale" null null)))
  (`KismetSystemLibrary.PrintString` "Done"))

(fn `UserConstructionScript`)