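; Platform actor that moves along a timeline-driven offset from its spawn location; despite the Destructable name, it contains no destruction logic.
; BeginPlay caches the location, then clears the Start flag after a FlatformStart delay.
; While Start is true, Tick calls Play on the timeline, whose updates set the actor location to the cached position plus the track value, without sweep.
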(event `self.ReceiveBeginPlay`
  ;[1 1 1] Start Trigger for Platform
  (set `self.Location` (`self.K2_GetActorLocation`))
  (`KismetSystemLibrary.Delay` (`self.Flatform_Start`))
  (set `self.Start` false))

(event `self.ReceiveTick`
  (params (DeltaSeconds :type "Float (single-precision)"))
  (if (`self.Start`)
    (`|ExecutionSequence`
      (:`then_0`
        (bind (_direction _newtrack_0) (`Timeline|Timeline_0`)
          (:`Update`
            (`self.K2_SetActorLocation` (+ _newtrack_0 (`self.Location`)))))))))

(fn `NewFunction_0`)

(fn `UserConstructionScript`)